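; Playable Susie character Blueprint for what appears to be a 2D fighter, handling movement, jumping and a light attack.
; Enhanced Input moves it along the Y axis, stopping instantly on release unless airborne.
; Jump and light-attack inputs jump the animation state machine to matching nodes.
; A separate Light event sphere-traces forward using DataTable range and radius, sending damage to the hit actor; other attacks and TakeDamage are empty.
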(event Custom|Light
  (bind _returnvalue (Transformation|GetActorLocation))
  (bind _returnvalue_2 (Utilities|GetDataTableRow (Variables|Default|GetData%20Table) "Light")
    (:then
      (bind _outhit (Collision|SphereTraceByChannel _returnvalue (+ _returnvalue (* (Transformation|GetActorForwardVector) (.Distance (Utilities|Struct|BreakS_HB _returnvalue_2)))) (.Radius (Utilities|Struct|BreakS_HB _returnvalue_2)) "TraceTypeQuery1" false 0 "ForOneFrame" true "(R=1.000000,G=0.000000,B=0.000000,A=1.000000)" "(R=0.000000,G=1.000000,B=0.000000,A=1.000000)" 1.0))
      (Class|BPIDamagable|TakeDamage(Message) (.HitActor (Collision|BreakHitResult _outhit)) (.Damage (Utilities|Struct|BreakS_HB _returnvalue_2))))))

(event Input|EnhancedActionEvents|EnhancedInputActionIA_HeavyAttack
  (params (ActionValue :type Boolean) (ElapsedSeconds :type Float%20%28double-precision%29) (TriggeredSeconds :type Float%20%28double-precision%29) (InputAction :type Input%20Action%20Object%20Reference :default "/Game/Blueprints/Characters/Input/FighterControl/Inputs/IA_HeavyAttack.IA_HeavyAttack")))

(event Input|EnhancedActionEvents|EnhancedInputActionIA_Movement
  (params (ActionValue :type Float%20%28double-precision%29) (ElapsedSeconds :type Float%20%28double-precision%29) (TriggeredSeconds :type Float%20%28double-precision%29) (InputAction :type Input%20Action%20Object%20Reference :default "/Game/Blueprints/Characters/Input/FighterControl/Inputs/IA_Movement.IA_Movement"))
  (:Triggered
    (Pawn|Input|AddMovementInput "0.000000,-1.000000,0.000000" ActionValue false :!label _label))
  (:Ongoing
    (goto _label))
  (:Canceled
    (if (not (Variables|Default|GetIsJumping)) :!label _label_2
      (Components|Movement|StopMovementImmediately (Variables|Character|GetCharacterMovement))))
  (:Completed
    (goto _label_2)))

(event Input|EnhancedActionEvents|EnhancedInputActionIA_Jump
  (params (ActionValue :type Boolean) (ElapsedSeconds :type Float%20%28double-precision%29) (TriggeredSeconds :type Float%20%28double-precision%29) (InputAction :type Input%20Action%20Object%20Reference :default "/Game/Blueprints/Characters/Input/FighterControl/Inputs/IA_Jump.IA_Jump"))
  (Character|Jump)
  (Variables|Default|SetIsJumping true)
  (Class|PaperZDAnimInstance|JumptoNode (Variables|Default|GetAnim%20Instance) "Airborne" "None"))

(event Input|EnhancedActionEvents|EnhancedInputActionIA_LightAttack
  (params (ActionValue :type Boolean) (ElapsedSeconds :type Float%20%28double-precision%29) (TriggeredSeconds :type Float%20%28double-precision%29) (InputAction :type Input%20Action%20Object%20Reference :default "/Game/Blueprints/Characters/Input/FighterControl/Inputs/IA_LightAttack.IA_LightAttack"))
  (Class|PaperZDAnimInstance|JumptoNode (Variables|Default|GetAnim%20Instance) "Light" "None"))

(event Input|EnhancedActionEvents|EnhancedInputActionIA_MediumAttack
  (params (ActionValue :type Boolean) (ElapsedSeconds :type Float%20%28double-precision%29) (TriggeredSeconds :type Float%20%28double-precision%29) (InputAction :type Input%20Action%20Object%20Reference :default "/Game/Blueprints/Characters/Input/FighterControl/Inputs/IA_MediumAttack.IA_MediumAttack")))

(event Input|EnhancedActionEvents|EnhancedInputActionIA_Special
  (params (ActionValue :type Boolean) (ElapsedSeconds :type Float%20%28double-precision%29) (TriggeredSeconds :type Float%20%28double-precision%29) (InputAction :type Input%20Action%20Object%20Reference :default "/Game/Blueprints/Characters/Input/FighterControl/Inputs/IA_Special.IA_Special")))

(event Input|EnhancedActionEvents|EnhancedInputActionIA_MoveLeft
  (params (ActionValue :type Float%20%28double-precision%29) (ElapsedSeconds :type Float%20%28double-precision%29) (TriggeredSeconds :type Float%20%28double-precision%29) (InputAction :type Input%20Action%20Object%20Reference :default "/Game/Blueprints/Characters/Input/FighterControl/Inputs/IA_MoveLeft.IA_MoveLeft"))
  (:Triggered
    (Pawn|Input|AddMovementInput "0.000000,1.000000,0.000000" ActionValue false :!label _label))
  (:Ongoing
    (goto _label))
  (:Canceled
    (if (not (Variables|Default|GetIsJumping)) :!label _label_2
      (Components|Movement|StopMovementImmediately (Variables|Character|GetCharacterMovement))))
  (:Completed
    (goto _label_2)))

(event Input|EnhancedActionEvents|EnhancedInputActionIA_MoveRight
  (params (ActionValue :type Float%20%28double-precision%29) (ElapsedSeconds :type Float%20%28double-precision%29) (TriggeredSeconds :type Float%20%28double-precision%29) (InputAction :type Input%20Action%20Object%20Reference :default "/Game/Blueprints/Characters/Input/FighterControl/Inputs/IA_MoveRight.IA_MoveRight"))
  (:Triggered
    (Pawn|Input|AddMovementInput "0.000000,-1.000000,0.000000" ActionValue false :!label _label))
  (:Ongoing
    (goto _label))
  (:Canceled
    (if (not (Variables|Default|GetIsJumping)) :!label _label_2
      (Components|Movement|StopMovementImmediately (Variables|Character|GetCharacterMovement))))
  (:Completed
    (goto _label_2)))

(event EventBeginPlay
  (bind _output_get (Variables|Default|SetAnim%20Instance (Variables|/Script/PaperZD.PaperZDAnimationComponent|GetAnimInstance (Variables|Default|GetAnimationComponent))))
  (Class|BPIAnimationBlueprintInterface|SetOwner(Message) _output_get))

(event Collision|EventActorBeginOverlap
  (params (OtherActor :type Actor%20Object%20Reference)))

(event EventTick
  (params (DeltaSeconds :type Float%20%28single-precision%29)))

(event EventOnLanded
  (params (Hit :type Hit%20Result%20Structure%20%28by%20ref%29))
  (Variables|Default|SetIsJumping false))

(event EventTakeDamage
  (params (DamageApplied :type Float%20%28double-precision%29)))

(fn ConstructionScript)