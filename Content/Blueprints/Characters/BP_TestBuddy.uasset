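; BP_TestBuddy is a test fighter character that moves along the world Y axis, jumps and performs light attacks.
; Enhanced Input drives movement, stopping it instantly on release unless airborne.
; Jump and light attack drive the PaperZD animation instance through JumpToNode, with jump and landing also updating ABP_Susie's Grounded flag.
; Dash, medium, heavy and special inputs, plus the DamageApplied event, are empty stubs.
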(event Custom|CustomEvent
  (params (DamageApplied :type Float%20%28double-precision%29)))

(event Input|EnhancedActionEvents|EnhancedInputActionIA_HeavyAttack
  (params (ActionValue :type Boolean) (ElapsedSeconds :type Float%20%28double-precision%29) (TriggeredSeconds :type Float%20%28double-precision%29) (InputAction :type Input%20Action%20Object%20Reference :default "/Game/Blueprints/Characters/Input/FighterControl/Inputs/IA_HeavyAttack.IA_HeavyAttack")))

(event Input|EnhancedActionEvents|EnhancedInputActionIA_Movement
  (params (ActionValue :type Float%20%28double-precision%29) (ElapsedSeconds :type Float%20%28double-precision%29) (TriggeredSeconds :type Float%20%28double-precision%29) (InputAction :type Input%20Action%20Object%20Reference :default "/Game/Blueprints/Characters/Input/FighterControl/Inputs/IA_Movement.IA_Movement"))
  (:Triggered
    (Pawn|Input|AddMovementInput "0.000000,-1.000000,0.000000" ActionValue false :!label _label))
  (:Ongoing
    (goto _label))
  (:Canceled
    (if (not (Variables|Default|GetIsJumping)) :!label _label_2
      (Components|Movement|StopMovementImmediately (Variables|Character|GetCharacterMovement))))
  (:Completed
    (goto _label_2)))

(event Input|EnhancedActionEvents|EnhancedInputActionIA_Jump
  (params (ActionValue :type Boolean) (ElapsedSeconds :type Float%20%28double-precision%29) (TriggeredSeconds :type Float%20%28double-precision%29) (InputAction :type Input%20Action%20Object%20Reference :default "/Game/Blueprints/Characters/Input/FighterControl/Inputs/IA_Jump.IA_Jump"))
  (bind _anim_instance (Variables|Default|GetAnim%20Instance))
  (Character|Jump)
  (Variables|Default|SetIsJumping true)
  (Class|PaperZDAnimInstance|JumptoNode _anim_instance "Airborne" "None")
  (bind _asabp_susie (Utilities|Casting|CastToABP_Susie _anim_instance))
  (bind _output_get (Variables|/Game/Characters/SusieSaute/ABP_Susie.ABP_Susie_C|SetGrounded _asabp_susie false))
  (Variables|/Game/Characters/SusieSaute/ABP_Susie.ABP_Susie_C|SetAttacking _asabp_susie _output_get))

(event Input|EnhancedActionEvents|EnhancedInputActionIA_LightAttack
  (params (ActionValue :type Boolean) (ElapsedSeconds :type Float%20%28double-precision%29) (TriggeredSeconds :type Float%20%28double-precision%29) (InputAction :type Input%20Action%20Object%20Reference :default "/Game/Blueprints/Characters/Input/FighterControl/Inputs/IA_LightAttack.IA_LightAttack"))
  (if (Variables|Default|GetIsCancelable)
    (if (Variables|Default|GetIsJumping)
      (Class|PaperZDAnimInstance|JumptoNode (Variables|Default|GetAnim%20Instance) "LightAir" "None")
      (else
        (Class|PaperZDAnimInstance|JumptoNode (Variables|Default|GetAnim%20Instance) "Light" "None")))))

(event Input|EnhancedActionEvents|EnhancedInputActionIA_MediumAttack
  (params (ActionValue :type Boolean) (ElapsedSeconds :type Float%20%28double-precision%29) (TriggeredSeconds :type Float%20%28double-precision%29) (InputAction :type Input%20Action%20Object%20Reference :default "/Game/Blueprints/Characters/Input/FighterControl/Inputs/IA_MediumAttack.IA_MediumAttack")))

(event Input|EnhancedActionEvents|EnhancedInputActionIA_Special
  (params (ActionValue :type Boolean) (ElapsedSeconds :type Float%20%28double-precision%29) (TriggeredSeconds :type Float%20%28double-precision%29) (InputAction :type Input%20Action%20Object%20Reference :default "/Game/Blueprints/Characters/Input/FighterControl/Inputs/IA_Special.IA_Special")))

(event Input|EnhancedActionEvents|EnhancedInputActionIA_MoveLeft
  (params (ActionValue :type Float%20%28double-precision%29) (ElapsedSeconds :type Float%20%28double-precision%29) (TriggeredSeconds :type Float%20%28double-precision%29) (InputAction :type Input%20Action%20Object%20Reference :default "/Game/Blueprints/Characters/Input/FighterControl/Inputs/IA_MoveLeft.IA_MoveLeft"))
  (:Triggered
    (Pawn|Input|AddMovementInput "0.000000,1.000000,0.000000" ActionValue false :!label _label))
  (:Ongoing
    (goto _label))
  (:Canceled
    (if (not (Variables|Default|GetIsJumping)) :!label _label_2
      (Components|Movement|StopMovementImmediately (Variables|Character|GetCharacterMovement))))
  (:Completed
    (goto _label_2)))

(event Input|EnhancedActionEvents|EnhancedInputActionIA_MoveRight
  (params (ActionValue :type Float%20%28double-precision%29) (ElapsedSeconds :type Float%20%28double-precision%29) (TriggeredSeconds :type Float%20%28double-precision%29) (InputAction :type Input%20Action%20Object%20Reference :default "/Game/Blueprints/Characters/Input/FighterControl/Inputs/IA_MoveRight.IA_MoveRight"))
  (:Triggered
    (Pawn|Input|AddMovementInput "0.000000,-1.000000,0.000000" ActionValue false :!label _label))
  (:Ongoing
    (goto _label))
  (:Canceled
    (if (not (Variables|Default|GetIsJumping)) :!label _label_2
      (Components|Movement|StopMovementImmediately (Variables|Character|GetCharacterMovement))))
  (:Completed
    (goto _label_2)))

(event Input|EnhancedActionEvents|EnhancedInputActionIA_DashForward
  (params (ActionValue :type Boolean) (ElapsedSeconds :type Float%20%28double-precision%29) (TriggeredSeconds :type Float%20%28double-precision%29) (InputAction :type Input%20Action%20Object%20Reference :default "/Game/Blueprints/Characters/Input/FighterControl/Inputs/IA_DashForward.IA_DashForward")))

(event EventBeginPlay
  (|CallParentFunction)
  (Variables|Default|SetAnim%20Instance (Variables|/Script/PaperZD.PaperZDAnimationComponent|GetAnimInstance (Variables|Default|GetAnimationComponent))))

(event EventTick
  (params (DeltaSeconds :type Float%20%28single-precision%29)))

(event EventOnLanded
  (params (Hit :type Hit%20Result%20Structure%20%28by%20ref%29))
  (Variables|Default|SetIsJumping false)
  (bind _asabp_susie (Utilities|Casting|CastToABP_Susie (Variables|Default|GetAnim%20Instance)))
  (bind _output_get (Variables|/Game/Characters/SusieSaute/ABP_Susie.ABP_Susie_C|SetGrounded _asabp_susie true))
  (Variables|Default|SetIsDashing _output_get))

(fn ConstructionScript
  (|CallParentFunction))