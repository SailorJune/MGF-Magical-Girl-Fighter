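; BP_CharacterCore is a character Blueprint with single-axis movement, GAS-driven jumping and an early attack setup.
; On BeginPlay, a data table row supplies the anim instance class and a grounded effect is applied.
; Movement input stops instantly on release unless jumping; landing also stops movement and, after a short delay, restores grounded state.
; The Light event sphere-traces forward with data-table values to send damage; attack inputs and TakeDamage are empty stubs.
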(event Custom|Light
  (bind _returnvalue (Transformation|GetActorLocation))
  (bind _returnvalue_2 (Utilities|GetDataTableRow (Variables|Default|GetData%20Table) "Light")
    (:then
      (Development|PrintString (Utilities|String|ToString(Vector) _returnvalue))
      (bind _outhit (Collision|SphereTraceByChannel _returnvalue (+ _returnvalue (* (Transformation|GetActorForwardVector) (.Distance (Utilities|Struct|BreakS_HB _returnvalue_2)))) (.Radius (Utilities|Struct|BreakS_HB _returnvalue_2)) "TraceTypeQuery1" false 0 "ForDuration" true "(R=1.000000,G=0.000000,B=0.000000,A=1.000000)" "(R=0.000000,G=1.000000,B=0.000000,A=1.000000)" 1e+01))
      (Class|BPIDamagable|TakeDamage(Message) (.HitActor (Collision|BreakHitResult _outhit)) (.Damage (Utilities|Struct|BreakS_HB _returnvalue_2))))))

(event Input|EnhancedActionEvents|EnhancedInputActionIA_HeavyAttack
  (params (ActionValue :type Boolean) (ElapsedSeconds :type Float%20%28double-precision%29) (TriggeredSeconds :type Float%20%28double-precision%29) (InputAction :type Input%20Action%20Object%20Reference :default "/Game/Blueprints/Characters/Input/FighterControl/Inputs/IA_HeavyAttack.IA_HeavyAttack")))

(event Input|EnhancedActionEvents|EnhancedInputActionIA_Movement
  (params (ActionValue :type Float%20%28double-precision%29) (ElapsedSeconds :type Float%20%28double-precision%29) (TriggeredSeconds :type Float%20%28double-precision%29) (InputAction :type Input%20Action%20Object%20Reference :default "/Game/Blueprints/Characters/Input/FighterControl/Inputs/IA_Movement.IA_Movement"))
  (:Triggered
    (Pawn|Input|AddMovementInput "0.000000,-1.000000,0.000000" ActionValue false :!label _label))
  (:Ongoing
    (goto _label))
  (:Canceled
    (if (not (Variables|Default|GetIsJumping)) :!label _label_2
      (Components|Movement|StopMovementImmediately (Variables|Character|GetCharacterMovement))))
  (:Completed
    (goto _label_2)))

(event Input|EnhancedActionEvents|EnhancedInputActionIA_Jump
  (params (ActionValue :type Boolean) (ElapsedSeconds :type Float%20%28double-precision%29) (TriggeredSeconds :type Float%20%28double-precision%29) (InputAction :type Input%20Action%20Object%20Reference :default "/Game/Blueprints/Characters/Input/FighterControl/Inputs/IA_Jump.IA_Jump"))
  (Abilities|TryActivateAbilitybyClass (Variables|Default|GetAbilitySystemComponent) (Variables|Default|GetJump%20Ability%20Container) true))

(event Input|EnhancedActionEvents|EnhancedInputActionIA_LightAttack
  (params (ActionValue :type Boolean) (ElapsedSeconds :type Float%20%28double-precision%29) (TriggeredSeconds :type Float%20%28double-precision%29) (InputAction :type Input%20Action%20Object%20Reference :default "/Game/Blueprints/Characters/Input/FighterControl/Inputs/IA_LightAttack.IA_LightAttack")))

(event Input|EnhancedActionEvents|EnhancedInputActionIA_MediumAttack
  (params (ActionValue :type Boolean) (ElapsedSeconds :type Float%20%28double-precision%29) (TriggeredSeconds :type Float%20%28double-precision%29) (InputAction :type Input%20Action%20Object%20Reference :default "/Game/Blueprints/Characters/Input/FighterControl/Inputs/IA_MediumAttack.IA_MediumAttack")))

(event Input|EnhancedActionEvents|EnhancedInputActionIA_Special
  (params (ActionValue :type Boolean) (ElapsedSeconds :type Float%20%28double-precision%29) (TriggeredSeconds :type Float%20%28double-precision%29) (InputAction :type Input%20Action%20Object%20Reference :default "/Game/Blueprints/Characters/Input/FighterControl/Inputs/IA_Special.IA_Special")))

(event Input|EnhancedActionEvents|EnhancedInputActionIA_MoveLeft
  (params (ActionValue :type Float%20%28double-precision%29) (ElapsedSeconds :type Float%20%28double-precision%29) (TriggeredSeconds :type Float%20%28double-precision%29) (InputAction :type Input%20Action%20Object%20Reference :default "/Game/Blueprints/Characters/Input/FighterControl/Inputs/IA_MoveLeft.IA_MoveLeft"))
  (:Triggered
    (Pawn|Input|AddMovementInput "0.000000,1.000000,0.000000" ActionValue false :!label _label))
  (:Ongoing
    (goto _label))
  (:Canceled
    (if (not (Variables|Default|GetIsJumping)) :!label _label_2
      (Components|Movement|StopMovementImmediately (Variables|Character|GetCharacterMovement))))
  (:Completed
    (goto _label_2)))

(event Input|EnhancedActionEvents|EnhancedInputActionIA_MoveRight
  (params (ActionValue :type Float%20%28double-precision%29) (ElapsedSeconds :type Float%20%28double-precision%29) (TriggeredSeconds :type Float%20%28double-precision%29) (InputAction :type Input%20Action%20Object%20Reference :default "/Game/Blueprints/Characters/Input/FighterControl/Inputs/IA_MoveRight.IA_MoveRight"))
  (:Triggered
    (Pawn|Input|AddMovementInput "0.000000,-1.000000,0.000000" ActionValue false :!label _label))
  (:Ongoing
    (goto _label))
  (:Canceled
    (if (not (Variables|Default|GetIsJumping)) :!label _label_2
      (Components|Movement|StopMovementImmediately (Variables|Character|GetCharacterMovement))))
  (:Completed
    (goto _label_2)))

(event EventBeginPlay
  (bind _abilitysystemcomponent (Variables|Default|GetAbilitySystemComponent))
  (bind _animationcomponent (Variables|Default|GetAnimationComponent))
  (bind _characterdata (Variables|Default|GetCharacterData))
  (bind _returnvalue (Utilities|GetDataTableRow (.datatable _characterdata) (.rowname _characterdata))
    (:then
      (Class|PaperZDAnimationComponent|SetAnimInstanceClass _animationcomponent (Utilities|Struct|BreakS_CharacterData _returnvalue))
      (Variables|Default|SetAnimationBlueprintInstance (Variables|/Script/PaperZD.PaperZDAnimationComponent|GetAnimInstance _animationcomponent))
      (GameplayEffects|ApplyGameplayEffectToSelf :self _abilitysystemcomponent :GameplayEffectClass "/Game/Blueprints/Characters/CharacterData/GameplayEffects/GE_IsGrounded.GE_IsGrounded_C" :Level 1.0)
      (GameplayEffects|RemoveActiveEffectswithGrantedTags _abilitysystemcomponent "(GameplayTags=((TagName=\"PlayerMovement.Jumping\")))"))))

(event EventOnLanded
  (params (Hit :type Hit%20Result%20Structure%20%28by%20ref%29))
  (bind _abilitysystemcomponent (Variables|Default|GetAbilitySystemComponent))
  (Components|Movement|StopMovementImmediately (Variables|Character|GetCharacterMovement))
  (Variables|Default|SetIsJumping false)
  (Utilities|FlowControl|Delay 0.1)
  (GameplayEffects|ApplyGameplayEffectToSelf :self _abilitysystemcomponent :GameplayEffectClass "/Game/Blueprints/Characters/CharacterData/GameplayEffects/GE_IsGrounded.GE_IsGrounded_C" :Level 1.0)
  (GameplayEffects|RemoveActiveEffectswithGrantedTags _abilitysystemcomponent "(GameplayTags=((TagName=\"PlayerMovement.Jumping\")))"))

(event EventTakeDamage
  (params (DamageApplied :type Float%20%28double-precision%29)))

(fn ConstructionScript)