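; Player character that moves along the world Y axis, with jumping driven by the Gameplay Ability System.
; BeginPlay sets the animation blueprint from a data table row and passes itself to it through an interface.
; Enhanced Input drives movement, stopping it on release unless jumping, and activates jump abilities by tag; attack and special inputs are empty stubs.
; Landing stops movement, applies the grounded effect and removes jumping effects.
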(event Input|EnhancedActionEvents|EnhancedInputActionIA_HeavyAttack
  (params (ActionValue :type Boolean) (ElapsedSeconds :type Float%20%28double-precision%29) (TriggeredSeconds :type Float%20%28double-precision%29) (InputAction :type Input%20Action%20Object%20Reference :default "/Game/Blueprints/Characters/Input/FighterControl/Inputs/IA_HeavyAttack.IA_HeavyAttack")))

(event Input|EnhancedActionEvents|EnhancedInputActionIA_Movement
  (params (ActionValue :type Float%20%28double-precision%29) (ElapsedSeconds :type Float%20%28double-precision%29) (TriggeredSeconds :type Float%20%28double-precision%29) (InputAction :type Input%20Action%20Object%20Reference :default "/Game/Blueprints/Characters/Input/FighterControl/Inputs/IA_Movement.IA_Movement"))
  (:Triggered
    (Pawn|Input|AddMovementInput "0.000000,-1.000000,0.000000" ActionValue false :!label _label))
  (:Ongoing
    (goto _label))
  (:Canceled
    (if (not (Variables|Default|GetIsJumping)) :!label _label_2
      (Components|Movement|StopMovementImmediately (Variables|Character|GetCharacterMovement))))
  (:Completed
    (goto _label_2)))

(event Input|EnhancedActionEvents|EnhancedInputActionIA_Jump
  (params (ActionValue :type Boolean) (ElapsedSeconds :type Float%20%28double-precision%29) (TriggeredSeconds :type Float%20%28double-precision%29) (InputAction :type Input%20Action%20Object%20Reference :default "/Game/Blueprints/Characters/Input/FighterControl/Inputs/IA_Jump.IA_Jump"))
  (Abilities|TryActivateAbilitiesbyTag (Variables|Default|GetAbilitySystemComponent) (Variables|Default|GetJump%20Tag%20Container) true))

(event Input|EnhancedActionEvents|EnhancedInputActionIA_LightAttack
  (params (ActionValue :type Boolean) (ElapsedSeconds :type Float%20%28double-precision%29) (TriggeredSeconds :type Float%20%28double-precision%29) (InputAction :type Input%20Action%20Object%20Reference :default "/Game/Blueprints/Characters/Input/FighterControl/Inputs/IA_LightAttack.IA_LightAttack")))

(event Input|EnhancedActionEvents|EnhancedInputActionIA_MediumAttack
  (params (ActionValue :type Boolean) (ElapsedSeconds :type Float%20%28double-precision%29) (TriggeredSeconds :type Float%20%28double-precision%29) (InputAction :type Input%20Action%20Object%20Reference :default "/Game/Blueprints/Characters/Input/FighterControl/Inputs/IA_MediumAttack.IA_MediumAttack")))

(event Input|EnhancedActionEvents|EnhancedInputActionIA_Special
  (params (ActionValue :type Boolean) (ElapsedSeconds :type Float%20%28double-precision%29) (TriggeredSeconds :type Float%20%28double-precision%29) (InputAction :type Input%20Action%20Object%20Reference :default "/Game/Blueprints/Characters/Input/FighterControl/Inputs/IA_Special.IA_Special")))

(event Input|EnhancedActionEvents|EnhancedInputActionIA_MoveLeft
  (params (ActionValue :type Float%20%28double-precision%29) (ElapsedSeconds :type Float%20%28double-precision%29) (TriggeredSeconds :type Float%20%28double-precision%29) (InputAction :type Input%20Action%20Object%20Reference :default "/Game/Blueprints/Characters/Input/FighterControl/Inputs/IA_MoveLeft.IA_MoveLeft"))
  (:Triggered
    (Pawn|Input|AddMovementInput "0.000000,1.000000,0.000000" ActionValue false :!label _label))
  (:Ongoing
    (goto _label))
  (:Canceled
    (if (not (Variables|Default|GetIsJumping)) :!label _label_2
      (Components|Movement|StopMovementImmediately (Variables|Character|GetCharacterMovement))))
  (:Completed
    (goto _label_2)))

(event Input|EnhancedActionEvents|EnhancedInputActionIA_MoveRight
  (params (ActionValue :type Float%20%28double-precision%29) (ElapsedSeconds :type Float%20%28double-precision%29) (TriggeredSeconds :type Float%20%28double-precision%29) (InputAction :type Input%20Action%20Object%20Reference :default "/Game/Blueprints/Characters/Input/FighterControl/Inputs/IA_MoveRight.IA_MoveRight"))
  (:Triggered
    (Pawn|Input|AddMovementInput "0.000000,-1.000000,0.000000" ActionValue false :!label _label))
  (:Ongoing
    (goto _label))
  (:Canceled
    (if (not (Variables|Default|GetIsJumping)) :!label _label_2
      (Components|Movement|StopMovementImmediately (Variables|Character|GetCharacterMovement))))
  (:Completed
    (goto _label_2)))

(event EventBeginPlay
  (bind _animationcomponent (Variables|Default|GetAnimationComponent))
  (bind _abilitysystemcomponent (Variables|Default|GetAbilitySystemComponent))
  (bind _characterdata (Variables|Default|GetCharacterData))
  (bind _returnvalue (Utilities|GetDataTableRow (.datatable _characterdata) (.rowname _characterdata))
    (:then
      (Class|PaperZDAnimationComponent|SetAnimInstanceClass _animationcomponent (.AnimationBlueprint (Utilities|Struct|BreakS_CharacterData _returnvalue)))
      (bind _output_get (Variables|Default|SetAnimationBlueprintInstance (Variables|/Script/PaperZD.PaperZDAnimationComponent|GetAnimInstance _animationcomponent)))
      (if (Utilities|DoesObjectImplementInterface _output_get "/Game/Blueprints/Interfaces/BPI_AnimationBlueprintInterface.BPI_AnimationBlueprintInterface_C")
        (Class|BPIAnimationBlueprintInterface|SetOwner(Message) _output_get self)
        (GameplayEffects|ApplyGameplayEffectToSelf :self _abilitysystemcomponent :GameplayEffectClass "/Game/Blueprints/Characters/CharacterData/GameplayEffects/GE_IsGrounded.GE_IsGrounded_C" :Level 1.0)
        (GameplayEffects|RemoveActiveEffectswithGrantedTags _abilitysystemcomponent "(GameplayTags=((TagName=\"PlayerMovement.Jumping\")))")
        (else
          (Development|PrintText "Please Implement the BPI_AnimationBlueprintInterface" true true "(R=0.000000,G=0.660000,B=1.000000,A=1.000000)" 1e+01))))))

(event EventOnLanded
  (params (Hit :type Hit%20Result%20Structure%20%28by%20ref%29))
  (bind _abilitysystemcomponent (Variables|Default|GetAbilitySystemComponent))
  (Variables|Default|SetIsJumping false)
  (Components|Movement|StopMovementImmediately (Variables|Character|GetCharacterMovement))
  (GameplayEffects|ApplyGameplayEffectToSelf :self _abilitysystemcomponent :GameplayEffectClass "/Game/Blueprints/Characters/CharacterData/GameplayEffects/GE_IsGrounded.GE_IsGrounded_C" :Level 1.0)
  ;[0.15 0.15 0.15 0.5] Will change to remove effect either after a brief delay or landing animation has ended
  (GameplayEffects|RemoveActiveEffectswithGrantedTags _abilitysystemcomponent "(GameplayTags=((TagName=\"PlayerMovement.Jumping\")))"))

(fn ConstructionScript)