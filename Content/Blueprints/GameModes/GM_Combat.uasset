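; GM_Combat is a combat game mode that spawns fighters for local players when play begins.
; It spawns a BP_TestBuddy at every PlayerStart, then has the player controller with the matching index possess it after adding the IM_Fighter input mapping context.
; Starts without a connected controller still get a pawn, and a message prints the missing index.
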(event EventBeginPlay
  (bind _outactors (Actor|GetAllActorsOfClass "/Script/Engine.PlayerStart"))
  (for (_array_element _array_index) _outactors
    (bind _returnvalue (Game|SpawnActorfromClass "/Game/Blueprints/Characters/BP_TestBuddy.BP_TestBuddy_C" (Transformation|GetActorTransform _array_element) "Undefined" "MultiplyWithRoot" _array_element 0))
    (Utilities|IsValid (Game|GetPlayerController _array_index)
      (:Is%20Valid
        (Input|AddMappingContext (PlayerController|LocalPlayerSubsystems|GetEnhancedInputLocalPlayerSubsystem (Game|GetPlayerController _array_index)) "/Game/Blueprints/Characters/Input/FighterControl/IM_Fighter.IM_Fighter" 0 "(bIgnoreAllPressedKeysUntilRelease=True,bForceImmediately=False,bNotifyUserSettings=False)")
        (Pawn|Possess (Game|GetPlayerController _array_index) _returnvalue))
      (:Is%20Not%20Valid
        (Development|PrintText (Utilities|Text|FormatText "No controller {index} connected!" _array_index))))))

(fn ConstructionScript)