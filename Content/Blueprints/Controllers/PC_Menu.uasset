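; PC_Menu is the player controller for the main menu, showing W_MainMenu with UI-only input and a visible cursor.
; On BeginPlay it also loads and applies saved game user settings and sets SCM_MGF as the base sound mix.
; If a sound settings save exists, its master, music and SFX volumes override that mix.
; An unconnected branch for registering the IM_Fighter mapping context with Enhanced Input user settings never runs.
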(event EventBeginPlay
  ;[0.15 0.15 0.15 0.5] Menu + Input Mode
  (bind _returnvalue (UserInterface|CreateWidget "/Game/Widgets/W_MainMenu.W_MainMenu_C" self))
  (bind _output_get (Variables|Default|SetMainMenu _returnvalue))
  (UserInterface|Viewport|AddtoViewport _output_get 0)
  (Input|SetInputModeUIOnly self _output_get "DoNotLock" false)
  (Variables|Default|SetbShowMouseCursor true)
  ;[0.15 0.15 0.15 0.5] Load Settings
  (bind _returnvalue_2 (Settings|GetGameUserSettings))
  (Class|GameUserSettings|LoadSettings _returnvalue_2 false)
  (Class|GameUserSettings|ApplyResolutionSettings _returnvalue_2 false)
  (Class|GameUserSettings|ApplyNonResolutionSettings _returnvalue_2)
  ;[0.15 0.15 0.15 0.5] Set Sound Settings
  (Class|GameplayStatics|SetBaseSoundMix "/Game/Audio/Classes/SCM_MGF.SCM_MGF")
  (bind _returnvalue_3 (SaveGame|DoesSaveGameExist "playerSoundSettings"))
  (if _returnvalue_3
    (bind _returnvalue_4 (SaveGame|LoadGamefromSlot "playerSoundSettings"))
    (bind _assgo_sound_settings (Utilities|Casting|CastToSGO_SoundSettings _returnvalue_4))
    (bind _output_get_2 (Variables|Default|SetSoundSettings _assgo_sound_settings))
    (Audio|SetSoundMixClassOverride "/Game/Audio/Classes/SCM_MGF.SCM_MGF" "/Game/Audio/Classes/SC_SFX.SC_SFX" (Variables|/Game/Blueprints/SaveGames/SGO_SoundSettings.SGO_SoundSettings_C|GetSoundVolume _output_get_2) 1.0 1.0 true)
    (Audio|SetSoundMixClassOverride "/Game/Audio/Classes/SCM_MGF.SCM_MGF" "/Game/Audio/Classes/SC_Music.SC_Music" (Variables|/Game/Blueprints/SaveGames/SGO_SoundSettings.SGO_SoundSettings_C|GetMusicVolume _output_get_2) 1.0 1.0 true)
    (Audio|SetSoundMixClassOverride "/Game/Audio/Classes/SCM_MGF.SCM_MGF" "/Game/Audio/Classes/SC_Master.SC_Master" (Variables|/Game/Blueprints/SaveGames/SGO_SoundSettings.SGO_SoundSettings_C|GetMasterVolume _output_get_2) 1.0 1.0 true)))

(fn ConstructionScript)